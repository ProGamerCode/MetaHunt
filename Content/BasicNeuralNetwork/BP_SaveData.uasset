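; BP_SaveData holds neuron data for a basic neural network, apparently as its save data.
; Its Print function loops over the NeuronData array and prints one long-lived debug string per neuron.
; Each string reports the neuron's id, input count, bias, layer and whether it is an input or output.
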(fn `print`
  (for _array_element (`self.neuronData`)
    (bind (_id _inputids _weights _bias _layer _isinput _isouput) (break `/Game/BasicNeuralNetwork/neurons/S_OutputNeuronData` _array_element))
    (`KismetSystemLibrary.PrintString` null (`KismetStringLibrary.Concat_StrStr` "id: " (`KismetStringLibrary.Conv_IntToString` _id) ", inputs: " (`KismetStringLibrary.Conv_IntToString` (`KismetArrayLibrary.Array_Length` _inputids)) ", bias: " (`KismetStringLibrary.Conv_DoubleToString` _bias) ", layer: " (`KismetStringLibrary.Conv_IntToString` _layer) ", is input: " (`KismetStringLibrary.Conv_BoolToString` _isinput) ", is output: " (`KismetStringLibrary.Conv_BoolToString` _isouput)) true true (struct :`G` 0.66 :`B` 1.0 :`A` 1.0) 200.0)))