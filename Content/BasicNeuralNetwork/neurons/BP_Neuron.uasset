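; BP_Neuron is a neuron for a basic neural network, apparently a base class with placeholder functions for output, weight adjustment and reset.
; Setup stores its id, activation parameter P, input and output flags, and hidden layer number.
; ThroughActivation maps a value to between 0 and 1 with a sigmoid whose steepness is controlled by P.
; GetOutput returns zero, while AdjustWeights and Reset are empty.
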(fn `adjustWeights`
  (params (targetOutput :type "Float (double-precision)") (learningRate :type "Float (double-precision)") (EW :type "Float (double-precision)")))

(fn `GetOutput`
  (returns (output :type "Float (double-precision)"))
  (return 0.0))

(fn `reset`)

(fn `setup`
  (params (givenId :type Integer) (p :type "Float (double-precision)") (isInput :type Boolean) (isOutput :type Boolean) (hiddenLayer :type Integer))
  (set `self.id` givenId)
  (set `self.p` p)
  (set `self.isInput` isInput)
  (set `self.isOutput` isOutput)
  (set `self.hiddenLayerNumber` hiddenLayer))

(fn `throughActivation`
  (params (valueIn :type "Float (double-precision)"))
  (returns (valueOut :type "Float (double-precision)"))
  (return (/ 1.0 (+ 1.0 (`KismetMathLibrary.MultiplyMultiply_FloatFloat` 2.7183 (* (/ valueIn (`self.p`)) -1.0))))))