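; Neural network neuron, serving as output or hidden node, that computes its value and learns by backpropagation.
; GetOutput recursively pulls weighted input values, subtracts the bias, applies the activation and caches the result until Reset clears it up the chain.
; AdjustWeights derives a sigmoid-derivative error from the target or from summed downstream errors once all have reported.
; It updates its weights, not the bias, then passes error times updated weight to each input.
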(event EventAdjustWeights
  (params (targetOutput :type Float%20%28single-precision%29) (learningRate :type Float%20%28single-precision%29) (EW :type Float%20%28single-precision%29))
  (bind _outputvalue (Variables|Fleeting|GetoutputValue))
  (bind _outputvalue_2 (Variables|Fleeting|GetoutputValue))
  (if (Variables|Fleeting|Getprocessed)
    (Variables|Fleeting|SettargetOutput targetOutput)
    (Variables|Persistent|SetlearningRate learningRate)
    (Variables|Fleeting|Setew EW)
    ;[1 1 1] Is this an output neuron or a hidden layer neuron
    (if (== (Variables|Persistent|GetnumOfOutputs) 0)
      ;[1 1 1] Adjust the weight for End output layer neurons
      (Variables|Fleeting|SetE (* (- (Variables|Fleeting|GettargetOutput) _outputvalue) _outputvalue (- 1.0 _outputvalue)))
      (for (_array_element _array_index) (Variables|Persistent|Getweights)
        (bind _output (CallFunction|GetOutput (Utilities|Array|Get(acopy) (Variables|Persistent|Getinputs) _array_index)))
        (Utilities|Array|SetArrayElem (Variables|Persistent|Getweights) _array_index (+ _array_element (* (Variables|Persistent|GetlearningRate) (Variables|Fleeting|GetE) _output)) true)
        ;[1 1 1] Call the next neuron up
        (Default|AdjustWeights (Utilities|Array|Get(acopy) (Variables|Persistent|Getinputs) _array_index) 0.0 (Variables|Persistent|GetlearningRate) (* (Utilities|Array|Get(acopy) (Variables|Persistent|Getweights) _array_index) (Variables|Fleeting|GetE))))
      (else
        ;[1 1 1] Add the child neuron's error*weight to our error rate
        (Variables|Fleeting|SetE (+ (Variables|Fleeting|Getew) (Variables|Fleeting|GetE)))
        (Variables|Persistent|SethiddenLayerCount (+ (Variables|Persistent|GethiddenLayerCount) 1))
        ;[1 1 1] Check to see if all of our children have given us their error
        (if (== (Variables|Persistent|GetnumOfOutputs) (Variables|Persistent|GethiddenLayerCount))
          ;[1 1 1] We have all the error information we need to adjust our weights and pass it up
          (Variables|Fleeting|SetE (* _outputvalue_2 (- 1.0 _outputvalue_2) (Variables|Fleeting|GetE)))
          (for (_array_element_2 _array_index_2) (Variables|Persistent|Getweights)
            (bind _output_2 (CallFunction|GetOutput (Utilities|Array|Get(acopy) (Variables|Persistent|Getinputs) _array_index_2)))
            (Utilities|Array|SetArrayElem (Variables|Persistent|Getweights) _array_index_2 (+ _array_element_2 (* (Variables|Persistent|GetlearningRate) (Variables|Fleeting|GetE) _output_2)) true)
            ;[1 1 1] Call the next neuron up
            (Default|AdjustWeights (Utilities|Array|Get(acopy) (Variables|Persistent|Getinputs) _array_index_2) 1.0 (Variables|Persistent|GetlearningRate) (* (Utilities|Array|Get(acopy) (Variables|Persistent|Getweights) _array_index_2) (Variables|Fleeting|GetE)))))))))

(event EventReset
  ;[1 1 1] Reset the neuron
  (if (Variables|Fleeting|Getprocessed)
    (Variables|Fleeting|Setprocessed false)
    (Variables|Persistent|SethiddenLayerCount 0)
    (Variables|Fleeting|SetE 0.0)
    (for _array_element (Variables|Persistent|Getinputs)
      (Default|Reset _array_element))))

(fn GetOutput
  (if (Variables|Fleeting|Getprocessed)
    (return (Variables|Fleeting|GetoutputValue))
    (else
      (LocalVariables|SettotalSum 0.0)
      ;[1 1 1] Add up the sums*weights of the inputs
      (for (_array_element _array_index) (Variables|Persistent|Getinputs)
        (bind _output (CallFunction|GetOutput _array_element))
        (LocalVariables|SettotalSum (+ (* _output (Utilities|Array|Get(acopy) (Variables|Persistent|Getweights) _array_index)) (LocalVariables|GettotalSum))))
      ;[1 1 1] Add(well subtract) the bias
      (bind _output_get (LocalVariables|SettotalSum (- (LocalVariables|GettotalSum) (Variables|Persistent|Getbias))))
      (bind _valueout (CallFunction|ThroughActivation _output_get))
      (bind _output_get_2 (Variables|Fleeting|SetoutputValue _valueout))
      (Variables|Fleeting|Setprocessed true)
      (return _output_get_2))))